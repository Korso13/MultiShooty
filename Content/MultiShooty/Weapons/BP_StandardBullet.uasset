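; Standard projectile actor for a multiplayer shooter that damages player pawns and expires after a set lifetime.
; BeginPlay starts a one-shot TTL timer that destroys the bullet.
; Mesh overlaps are handled only on the server as cheat protection, passing the other actor to the server hit event.
; That event applies Damage through the HP component of any BP_MultiplayerPawnBase hit, then destroys the bullet whatever it struck.
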(event OnComponentBeginOverlap(BulletMesh)
  (params (OverlappedComponent :type Primitive%20Component%20Object%20Reference) (OtherActor :type Actor%20Object%20Reference) (OtherComp :type Primitive%20Component%20Object%20Reference) (OtherBodyIndex :type Integer) (bFromSweep :type Boolean) (SweepResult :type Hit%20Result%20Structure%20%28by%20ref%29))
  ;[0.5833 0.744 1] Bullet hit call
  ;;[0.28 1 0.9602] Cheating protection
  (if (Networking|IsServer)
    (CallFunction|ServerObjectHit OtherActor)))

(event Custom|BulletExpired
  ;[0.5833 0.744 1] Bullet expiration
  (Actor|DestroyActor))

(event Custom|Server_ObjectHit
  (params (HitActor :type Actor%20Object%20Reference))
  ;[0.5833 0.744 1] Bullet hit call
  ;;[1 0.3061 0.3959] Apply damage if possible, destroy bullet
  (bind _asbp_multiplayer_pawn_base (Utilities|Casting|CastToBP_MultiplayerPawnBase HitActor)
    (:then
      (Default|TakeDamage (Variables|/Game/MultiShooty/Pawns/BP_MultiplayerPawnBase.BP_MultiplayerPawnBase_C|GetMultiplayerHPComponent _asbp_multiplayer_pawn_base) (Variables|Default|GetDamage)))
    (:CastFailed
      _))
  (Actor|DestroyActor))

(event EventBeginPlay
  ;[0.5833 0.744 1] Bullet expiration
  (Utilities|Time|SetTimerbyEvent (delegate Custom|BulletExpired) (Variables|Default|GetTTL)))

(event Collision|EventActorBeginOverlap
  (params (OtherActor :type Actor%20Object%20Reference)))

(event EventTick
  (params (DeltaSeconds :type Float%20%28single-precision%29)))

(fn ConstructionScript)