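; Base multiplayer shooter pawn with axis movement, jumping, a held weapon, an overhead HP bar and team colors.
; BeginPlay attaches a temporary rifle to the hand socket, passes the HP bar widget to the HP component and, after a short delay, sets its initial fill.
; Fire input toggles a flag that Tick polls to call the weapon's ServerFire when it can fire.
; Events set the team material and overhead player name.
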(event Custom|Fire_Gun
  ;[0.3297 0.6319 1] Input setup
  ;;[1 0.3604 0.4302] Server-Replicated firing input
  (bind _activeweapon (Variables|Default|GetActiveWeapon)
    (:then
      (if (Variables|/Game/MultiShooty/Weapons/BP_ValRifle.BP_ValRifle_C|GetbCanFire _activeweapon)
        (Default|ServerFire (Variables|Default|GetActiveWeapon))))
    (:else)))

(event Custom|Set%20Team%20Colors
  (params (TeamID :type Byte))
  ;[1 0.2317 0.8643] Setting team color for this pawn
  (Rendering|Material|SetMaterial (Variables|Default|GetStaticMesh) 0 (Utilities|Select :Index TeamID :Option%200 "/Game/FPS_Weapon_Bundle/Weapons/Materials/Ammunition/M_45ap.M_45ap" :Option%201 "/Game/MultiShooty/Materials/M_Team1Colors.M_Team1Colors" :Option%202 "/Game/MultiShooty/Materials/M_Team2Colors.M_Team2Colors"))
  (Utilities|FlowControl|Delay 0.1))

(event Custom|Update_Nick
  (params (Nick :type Text))
  (bind _asw_overhead_hpwidget (Utilities|Casting|CastToW_OverheadHPWidget (UserInterface|GetWidget (Variables|Default|GetHP%20bar%20widget))))
  (Variables|/Game/MultiShooty/UI/W_OverheadHPWidget.W_OverheadHPWidget_C|SetW_PlayerName _asw_overhead_hpwidget (Variables|Default|GetP_PlayerName)))

(event EventBeginPlay
  (bind _multiplayerhpcomponent (Variables|Default|GetMultiplayerHPComponent))
  (bind _maxhp (Variables|/Game/MultiShooty/Components/BP_MultiplayerHPComponent.BP_MultiplayerHPComponent_C|GetMaxHP _multiplayerhpcomponent))
  (Utilities|FlowControl|Sequence
    (:then_0
      ;[1 1 1] Temp solution to add weapon in hands
      (bind _returnvalue (Game|SpawnActorfromClass "/Game/MultiShooty/Weapons/BP_ValRifle.BP_ValRifle_C" (Transformation|GetSocketTransform (Variables|Default|GetHands_SK) "hand_rSocket" "RTS_Actor") "AlwaysSpawn" 0 0))
      (bind _output_get (Variables|Default|SetActiveWeapon _returnvalue))
      (Transformation|AttachComponentToComponent _output_get (Variables|Default|GetHands_SK) "hand_rSocket" "SnapToTarget" "KeepRelative" "SnapToTarget" false)
      (Variables|/Game/MultiShooty/Weapons/BP_ValRifle.BP_ValRifle_C|SetOwningPawn (Variables|Default|GetActiveWeapon) self))
    (:then_1
      ;[0.2997 0.3041 1] Pass HPBar widget to HP Component
      (Variables|/Game/MultiShooty/Components/BP_MultiplayerHPComponent.BP_MultiplayerHPComponent_C|SetHPWidgetRef (Variables|Default|GetMultiplayerHPComponent) (Variables|Default|GetHP%20bar%20widget))
      (Utilities|FlowControl|Delay 0.1)
      ;[0.427 1 0.9901] Setting HP bar value on spawn
      (bind _asw_overhead_hpwidget (Utilities|Casting|CastToW_OverheadHPWidget (UserInterface|GetWidget (Variables|Default|GetHP%20bar%20widget))))
      (if (!= _maxhp 0.0)
        (Default|SetNewHP _asw_overhead_hpwidget (/ (Variables|/Game/MultiShooty/Components/BP_MultiplayerHPComponent.BP_MultiplayerHPComponent_C|GetCurrent%20HP _multiplayerhpcomponent) _maxhp))))))

(event Collision|EventActorBeginOverlap
  (params (OtherActor :type Actor%20Object%20Reference)))

(event EventTick
  (params (DeltaSeconds :type Float%20%28single-precision%29))
  ;[0.3297 0.6319 1] Input setup
  ;;[1 0.3604 0.4302] Server-Replicated firing input
  (if (Variables|Default|GetbFiring)
    (CallFunction|FireGun)))

(event Input|ActionEvents|InputActionJump
  (params (Key :type Key%20Structure :default "None"))
  ;[0.3297 0.6319 1] Input setup
  (:Pressed
    (Character|Jump))
  (:Released
    (Character|StopJumping)))

(event Input|ActionEvents|InputActionFire
  (params (Key :type Key%20Structure :default "None"))
  ;[0.3297 0.6319 1] Input setup
  ;;[1 0.3604 0.4302] Server-Replicated firing input
  (:Pressed
    (Variables|Default|SetbFiring true))
  (:Released
    (Variables|Default|SetbFiring false)))

(event Input|AxisEvents|InputAxisTurn
  (params (AxisValue :type Float%20%28single-precision%29))
  ;[0.3297 0.6319 1] Input setup
  (Pawn|Input|AddControllerYawInput AxisValue))

(event Input|AxisEvents|InputAxisLookUp
  (params (AxisValue :type Float%20%28single-precision%29))
  ;[0.3297 0.6319 1] Input setup
  (Pawn|Input|AddControllerPitchInput AxisValue))

(event Input|AxisEvents|InputAxisMoveForward
  (params (AxisValue :type Float%20%28single-precision%29))
  ;[0.3297 0.6319 1] Input setup
  ;;[1 0.3125 0.3125] Main axis movement
  (Pawn|Input|AddMovementInput (Math|Vector|GetForwardVector (Math|Rotator|MakeRotator 0.0 0.0 (.yaw (Pawn|GetControlRotation :!class /Script/Engine.Pawn)))) AxisValue false))

(event Input|AxisEvents|InputAxisMoveRight
  (params (AxisValue :type Float%20%28single-precision%29))
  ;[0.3297 0.6319 1] Input setup
  ;;[1 0.3125 0.3125] Main axis movement
  (Pawn|Input|AddMovementInput (Math|Vector|GetRightVector (Math|Rotator|MakeRotator 0.0 0.0 (.yaw (Pawn|GetControlRotation :!class /Script/Engine.Pawn)))) AxisValue false))

(fn ConstructionScript)