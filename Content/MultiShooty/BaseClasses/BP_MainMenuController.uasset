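; Player controller for the main menu that shows the W_MainMenu widget when play begins.
; BeginPlay calls a client open-menu event, so the server does not build menus for every player controller.
; That event creates the widget for this controller, adds it to the viewport, switches input to UI-only focused on it and shows the mouse cursor.
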(event Custom|Client_OpenMenu
  ;[1 1 1] Open main menu widget
  (bind _returnvalue (UserInterface|CreateWidget "/Game/MultiShooty/UI/W_MainMenu.W_MainMenu_C" self))
  (bind _output_get (Variables|Default|SetMenuWidget _returnvalue))
  (UserInterface|Viewport|AddtoViewport _output_get 0)
  (Input|SetInputModeUIOnly self (Variables|Default|GetMenuWidget) "DoNotLock")
  (Variables|/Script/Engine.PlayerController|SetbShowMouseCursor self true))

(event EventBeginPlay
  ;[1 0.5832 0.5932] Prevents server from initializing menu for all player controllers on server-side
  (CallFunction|ClientOpenMenu))

(event EventTick
  (params (DeltaSeconds :type Float%20%28single-precision%29)))

(fn ConstructionScript)