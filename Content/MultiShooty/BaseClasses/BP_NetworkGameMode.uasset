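; BP_NetworkGameMode is a multiplayer game mode that sorts joining players into two teams.
; PostLogin assigns the player controller to the smaller team, favoring Team1 on ties, with a generated team-and-number name.
; After a short delay, it calls RefreshColors on team controllers with their pawns so the newcomer sees correct team colors.
; Team membership lives in Teamless, Team1 and Team2 arrays selected by TeamID, and logout removes the player.
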(event EventBeginPlay)

(event EventTick
  (params (DeltaSeconds :type Float%20%28single-precision%29)))

(event EventPostLogin
  (params (NewPlayer :type Player%20Controller%20Object%20Reference))
  (bind _team1 (Variables|Default|GetTeam1))
  (bind _team2 (Variables|Default|GetTeam2))
  (bind _returnvalue (Utilities|Array|Length _team1))
  (bind _returnvalue_2 (Utilities|Array|Length _team2))
  (bind _returnvalue_3 (<= _returnvalue _returnvalue_2))
  (bind _returnvalue_4 (select _returnvalue_3 1 2))
  ;[1 0.5112 0.3808] Add player to either smallest or the first team
  (bind _asbp_multiplayer_player_controller (Utilities|Casting|CastToBP_MultiplayerPlayerController NewPlayer)
    (:then
      ;;[0.1367 0.3032 1] Set teamID and nickname tag in player controller
      (Variables|/Game/MultiShooty/BaseClasses/BP_MultiplayerPlayerController.BP_MultiplayerPlayerController_C|SetTeamID _asbp_multiplayer_player_controller _returnvalue_4)
      (Variables|/Game/MultiShooty/BaseClasses/BP_MultiplayerPlayerController.BP_MultiplayerPlayerController_C|SetPlayerName _asbp_multiplayer_player_controller (Utilities|String|Append "Team" (Utilities|String|ToString(Byte) _returnvalue_4) "_Player" (Utilities|String|ToString(Integer) (Utilities|Array|Length (Utilities|Select :Index _returnvalue_4 :Option%200 (Variables|Default|GetTeamless) :Option%201 (Variables|Default|GetTeam1) :Option%202 (Variables|Default|GetTeam2))))))
      (CallFunction|AddPlayertoTeam _asbp_multiplayer_player_controller _returnvalue_4)
      ;;[0.1679 0.2274 1] Sets correct team colors for newly-joined client
      (Utilities|FlowControl|Delay 0.2)
      (CallFunction|RefreshLocalPawnColors))
    (:CastFailed
      (Development|PrintString "Controller cast failed (On login)" true true "(R=1.000000,G=0.958173,B=0.095608,A=1.000000)"))))

(event EventOnLogout
  (params (ExitingController :type Controller%20Object%20Reference))
  ;[1 0.8959 0.3865] Remove player from team on logout
  (bind _asbp_multiplayer_player_controller (Utilities|Casting|CastToBP_MultiplayerPlayerController ExitingController))
  (CallFunction|RemovePlayerfromTeam _asbp_multiplayer_player_controller))

(fn ConstructionScript)

(fn AddPlayertoTeam
  (params (PlayerController :type BP%20Multiplayer%20Player%20Controller%20Object%20Reference) (TeamID :type Byte))
  (if (and (< TeamID 3) (>= TeamID 0))
    ;[0.0317 0.1963 1] Remove player from current team
    (Utilities|Array|RemoveItem (Variables|Default|GetTeamless) PlayerController)
    (Utilities|Array|RemoveItem (Variables|Default|GetTeam1) PlayerController)
    (Utilities|Array|RemoveItem (Variables|Default|GetTeam2) PlayerController)
    (Utilities|Array|Add (Utilities|Select :Index TeamID :Option%200 (Variables|Default|GetTeamless) :Option%201 (Variables|Default|GetTeam1) :Option%202 (Variables|Default|GetTeam2)) PlayerController)))

(fn RefreshLocalPawnColors
  (bind _team1 (Variables|Default|GetTeam1))
  (bind _team2 (Variables|Default|GetTeam2))
  ;[1 0.4145 0.3846] Cheching if there are any players on team 1
  (if (> (Utilities|Array|Length _team1) 0)
    (for _array_element _team1
      ;[0.03215 0.09719 1] Refreshing colors for team1
      ;;[1 1 1] Pawn controlled by player controller
      (bind _asbp_multiplayer_pawn_base (Utilities|Casting|CastToBP_MultiplayerPawnBase (Pawn|GetControlledPawn _array_element)))
      (Default|RefreshColors _array_element _asbp_multiplayer_pawn_base)))
  ;[1 0.4145 0.3846] Cheching if there are any players on team 2
  (if (> (Utilities|Array|Length _team2) 0)
    ;[0.03215 0.09719 1] Refreshing colors for team 2
    (for _array_element_2 _team2
      ;;[1 1 1] Pawn controlled by player controller
      (bind _asbp_multiplayer_pawn_base_2 (Utilities|Casting|CastToBP_MultiplayerPawnBase (Pawn|GetControlledPawn _array_element_2)))
      (Default|RefreshColors _array_element_2 _asbp_multiplayer_pawn_base_2))))

(fn RemovePlayerfromTeam
  (params (PlayerController :type BP%20Multiplayer%20Player%20Controller%20Object%20Reference))
  (Utilities|Array|RemoveItem (Utilities|Select :Index (Variables|/Game/MultiShooty/BaseClasses/BP_MultiplayerPlayerController.BP_MultiplayerPlayerController_C|GetTeamID PlayerController) :Option%200 (Variables|Default|GetTeamless) :Option%201 (Variables|Default|GetTeam1) :Option%202 (Variables|Default|GetTeam2)) PlayerController))