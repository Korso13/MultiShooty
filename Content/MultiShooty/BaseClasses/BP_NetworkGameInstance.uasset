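; Game instance Blueprint that handles multiplayer session hosting, searching and joining through the built-in async session nodes.
; Hosting creates a LAN or online session, then opens the chosen map as a listen server.
; Searching stores found sessions and passes them to the main menu, which supplies its own reference.
; Results, failures and network errors are reported as on-screen debug prints, with error messages using the last join target's details.
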(event Custom|Create%20New%20Session
  (params (MaxPlayers :type Integer) (bLAN :type Boolean) (MapName :type Name :default "Level1"))
  ;[0.4655 0.4928 1] Function creating new listenning server session
  (|Session (Game|GetPlayerController 0) MaxPlayers bLAN
    (:OnSuccess
      (Game|OpenLevel(byName) MapName true "listen"))
    (:OnFailure
      (Development|PrintString "Session creation failed!!!" true true "(R=1.000000,G=0.018600,B=0.000000,A=1.000000)"))))

(event Custom|GetServers
  (params (bSearchLAN :type Boolean) (MainMenuRef :type W%20Main%20Menu%20Object%20Reference))
  ;[0.3186 1 0.3008] Find sessions
  (bind _results (|FindSessions (Game|GetPlayerController 0) 5 bSearchLAN)
    (:OnSuccess
      (for _array_element _results
        (Development|PrintString (Utilities|String|Append "Server name: " (Class|FindSessionsCallbackProxy|GetServerName _array_element) " Players: " (Utilities|String|ToString(Integer) (Class|FindSessionsCallbackProxy|GetCurrentPlayers _array_element)) "/" (Utilities|String|ToString(Integer) (Class|FindSessionsCallbackProxy|GetMaxPlayers _array_element)) " Ping: " (Utilities|String|ToString(Integer) (Class|FindSessionsCallbackProxy|GetPinginMs _array_element)))))
      ;;[0.4161 0.2142 1] Return server search results to widget
      (bind _output_get (Variables|Default|SetFoundServersArray _results))
      ;;;[1 0 0.09242] Check if any servers were found
      (if (> (Utilities|Array|Length _output_get) 0)
        (Default|GetServerSearchResults MainMenuRef _output_get)))
    (:OnFailure
      (Development|PrintString "No servers found!" true true "(R=1.000000,G=0.008761,B=0.000000,A=1.000000)"))))

(event Custom|JoinSession
  (params (Server :type Blueprint%20Session%20Result%20Structure))
  ;[1 0.3541 0.364] Join session
  (|JoinSession (Game|GetPlayerController 0) Server
    (:OnFailure
      (Development|PrintString "Couldn't join the game!"))))

(event EventHandleNetworkError
  (params (FailureType :type ENetworkFailure%20Enum :default "NetDriverAlreadyExists") (bIsServer :type Boolean))
  ;[1 1 1] Network error debug message
  (Development|PrintString (Utilities|String|Append (select bIsServer "Server " "Client ") "error: " (Utilities|String|EnumtoString FailureType) ". Server name: " (Class|FindSessionsCallbackProxy|GetServerName (stale Custom|JoinSession Server)) ". Ping: " (Utilities|String|ToString(Integer) (Class|FindSessionsCallbackProxy|GetPinginMs (stale Custom|JoinSession Server))) " ms.") true true "(R=1.000000,G=0.207129,B=0.187233,A=1.000000)" 1e+01))