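; BP_ValRifle is a rifle weapon for MultiShooty that fires projectiles through server-named events.
; Server_Fire calls Fire, which spawns BulletClass at the Barrel's world location and rotation, with the owning pawn as owner and instigator.
; It then triggers a refire delay, commented as server-to-single-client, that clears CanFire until RefireTime elapses.
; Fire and Server_Fire do not check CanFire themselves.
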(event Custom|Server_Fire
  ;[0.5161 0.5103 1] Weapon fire call (serverside)
  (CallFunction|Fire)
  (CallFunction|ServerRefireDelay))

(event Custom|Server_RefireDelay
  ;[1 0.5426 0.9995] Refire enabling (server to single client)
  (Variables|Default|SetbCanFire false)
  (Utilities|FlowControl|Delay (Variables|Default|GetRefireTime))
  (Variables|Default|SetbCanFire true))

(event EventBeginPlay)

(event Collision|EventActorBeginOverlap
  (params (OtherActor :type Actor%20Object%20Reference)))

(event EventTick
  (params (DeltaSeconds :type Float%20%28single-precision%29)))

(fn ConstructionScript)

(fn Fire
  (bind _barrel (Variables|Default|GetBarrel))
  (bind _owningpawn (Variables|Default|GetOwningPawn))
  (Game|SpawnActorfromClass (Variables|Default|GetBulletClass) (Math|Transform|MakeTransform (Transformation|GetWorldLocation _barrel) (Transformation|GetWorldRotation _barrel)) "AlwaysSpawn" _owningpawn _owningpawn))