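; Player controller for multiplayer matches that handles game input mode, team colors and nametags, and leaving the session.
; On BeginPlay it switches to game-only input, then after a short delay multicasts team colors and the player's name to the controlled pawn.
; The Home key logs out through the network game mode on the server, then opens MainMenu and destroys the session on the client.
; A deprecated main menu path remains but is unused.
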(event Custom|Client_OpenMenu
  ;[0 0 0] DEPRICATED! Moved back to Main Menu Player Controller
  ;;[0.962 0.4921 1] Set UI-aimed controllerr scheme. Open main menu widget
  (bind _returnvalue (UserInterface|CreateWidget "/Game/MultiShooty/UI/W_MainMenu.W_MainMenu_C" self))
  (bind _output_get (Variables|Default|SetMenuWidget _returnvalue))
  (UserInterface|Viewport|AddtoViewport _output_get 0)
  (Input|SetInputModeUIOnly self (Variables|Default|GetMenuWidget) "DoNotLock")
  (Variables|/Script/Engine.PlayerController|SetbShowMouseCursor self true))

(event Custom|Client_SwitchToGameMode
  ;[0.962 0.4921 1] Seting regular game player controller
  (Input|SetInputModeGameOnly self)
  (Variables|Default|SetbShowMouseCursor false))

(event Custom|Server_logout
  (params (Player%20Controller :type Player%20Controller%20Object%20Reference))
  ;[1 0.02186 0] Logout on button "Home"
  (bind _asbp_network_game_mode (Utilities|Casting|CastToBP_NetworkGameMode (Game|GetGameMode)))
  (|Logout _asbp_network_game_mode Player%20Controller))

(event Custom|Client_logout
  ;[1 0.02186 0] Logout on button "Home"
  (Game|OpenLevel(byName) "MainMenu")
  (|DestroySession self))

(event Custom|Multicast_Set%20TeamID,%20Name%20and%20Colors
  ;[0.2842 1 0.2266] Team color and nametag setup
  ;;[1 0.9105 0.2188] Seting player's team colors and nametag upon spawn
  (bind _asbp_multiplayer_pawn_base (Utilities|Casting|CastToBP_MultiplayerPawnBase (Pawn|GetControlledPawn))
    (:then
      (Default|SetTeamColors _asbp_multiplayer_pawn_base (Variables|Default|GetTeamID))
      ;;;[1 0.477 0.8622] Replicated and used by each client's copy of pawn to set nametag
      (Variables|/Game/MultiShooty/Pawns/BP_MultiplayerPawnBase.BP_MultiplayerPawnBase_C|SetP_PlayerName _asbp_multiplayer_pawn_base (Utilities|Text|ToText(String) (Variables|Default|GetPlayerName))))
    (:CastFailed
      (Development|PrintString (Utilities|String|Append "Pawn cast failed" (Variables|Default|GetPlayerName))))))

(event Custom|RefreshColors
  (params (PawnReference :type BP%20Multiplayer%20Pawn%20Base%20Object%20Reference))
  ;[0.2842 1 0.2266] Team color and nametag setup
  ;;[1 0.01364 0] Called from server for each client to correctly set team colors for all
  (Default|SetTeamColors PawnReference (Variables|Default|GetTeamID)))

(event EventBeginPlay
  (Utilities|FlowControl|Sequence
    (:then_0
      (CallFunction|ClientSwitchtoGameMode))
    (:then_1
      ;[0.2842 1 0.2266] Team color and nametag setup
      ;;[1 1 1] Begin Play
      (Utilities|FlowControl|Delay 0.1)
      ;;[0.5948 0.2493 1] Set pawn's colors on spawn
      (CallFunction|MulticastSetTeamID,NameandColors))))

(event EventTick
  (params (DeltaSeconds :type Float%20%28single-precision%29)))

(event Input|KeyboardEvents|Home
  (params (Key :type Key%20Structure :default "None"))
  ;[1 0.02186 0] Logout on button "Home"
  (:Pressed
    (CallFunction|ServerLogout self)
    (Utilities|FlowControl|Delay 0.2)
    (CallFunction|ClientLogout)))

(fn ConstructionScript)